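; Chicken AI pawn that the player herds into a pen by ringing a bell.
; While the player is inside its PlayerSphere, it polls BellRung with a recursive short Delay, then uses AIMoveTo to flee directly away.
; It keeps fleeing while the player stays in range and it is not penned, otherwise idling once out of range.
; Overlapping a PenBlueprint marks it penned, triggers one more run and increments the player's PenPoints, printing a win at the target count.
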(event `self.ReceiveBeginPlay`
  ;[1 1 1] Referemces the character
  (bind _asfirst_person_character (cast `/Game/FirstPersonBP/Blueprints/FirstPersonCharacter` (`GameplayStatics.GetPlayerCharacter` 0)))
  (set `self.CharacterRef` _asfirst_person_character)
  (`SkeletalMeshComponent.PlayAnimation` (`self.Mesh`) "/Game/FarmAnimalsPack/Chicken/Animations/ANIM_Chicken_Idle1.ANIM_Chicken_Idle1" true))

(event `self.PlayerSphere.OnComponentBeginOverlap`
  (params (OverlappedComponent :type "PrimitiveComponent Object Reference") (OtherActor :type "Actor Object Reference") (OtherComp :type "PrimitiveComponent Object Reference") (OtherBodyIndex :type Integer) (bFromSweep :type Boolean) (SweepResult :type "HitResult Structure (by ref)"))
  ;[1 1 1] Checks if the player is nearby the AI, if so casts the bell check event and sets inside radius boolean to true.
  (cast `/Game/FirstPersonBP/Blueprints/FirstPersonCharacter` OtherActor)
  (set `self.Inside Radius` true)
  (if (not (`self.InsidePen`))
    ;[1 1 1] Checks if the player is no longer nearby the AI, if so sets the inside radius boolean to false.
    (`self.EventBellCheck`)))

(event `self.PlayerSphere.OnComponentEndOverlap`
  (params (OverlappedComponent :type "PrimitiveComponent Object Reference") (OtherActor :type "Actor Object Reference") (OtherComp :type "PrimitiveComponent Object Reference") (OtherBodyIndex :type Integer))
  ;[1 1 1] Checks if the player is no longer nearby the AI, if so sets the inside radius boolean to false.
  (cast `/Game/FirstPersonBP/Blueprints/FirstPersonCharacter` OtherActor)
  (set `self.Inside Radius` false))

(event `EventBellCheck`
  ;[1 1 1] While the player is nearby the ai it checks if the player has rung the bell yet. If they have then it will call the run away event
  (bind _asfirst_person_character (cast `/Game/FirstPersonBP/Blueprints/FirstPersonCharacter` (`GameplayStatics.GetPlayerCharacter` 0)))
  (if (`self.Inside Radius`)
    (if (`/Game/FirstPersonBP/Blueprints/FirstPersonCharacter.BellRung` _asfirst_person_character)
      (`self.Event RunAway`)
      (else
        (`KismetSystemLibrary.Delay` 0.01)
        (`self.EventBellCheck`)))))

(event `Event RunAway`
  (bind _returnvalue (`self.K2_GetActorLocation`))
  (bind _characterref (`self.CharacterRef`))
  ;[1 1 1] Makes the AI run away from the player.
  (`SkeletalMeshComponent.PlayAnimation` (`self.Mesh`) "/Game/FarmAnimalsPack/Chicken/Animations/ANIM_Chicken_Run.ANIM_Chicken_Run" true)
  (`/Engine/EditorBlueprintResources/StandardMacros.IsValid` _characterref
    (:`Is Valid`
      (`|AIMoveTo` self (`KismetMathLibrary.MakeVector` (.x (+ _returnvalue (* (`KismetMathLibrary.GetForwardVector` (`KismetMathLibrary.FindLookAtRotation` _returnvalue (`self.K2_GetActorLocation` _characterref))) -750.0))) (.y (+ _returnvalue (* (`KismetMathLibrary.GetForwardVector` (`KismetMathLibrary.FindLookAtRotation` _returnvalue (`self.K2_GetActorLocation` _characterref))) -750.0))) (.z _returnvalue)) null
        (:`OnSuccess`
          _)
        (:`OnFail`
          _))
      (if (`self.Inside Radius`)
        (if (not (`self.InsidePen`))
          (`self.Event RunAway`))
        (else
          (`SkeletalMeshComponent.PlayAnimation` (`self.Mesh`) "/Game/FarmAnimalsPack/Chicken/Animations/ANIM_Chicken_Idle1.ANIM_Chicken_Idle1" true))))))

(event `self.PenSphere.OnComponentBeginOverlap`
  (params (OverlappedComponent :type "PrimitiveComponent Object Reference") (OtherActor :type "Actor Object Reference") (OtherComp :type "PrimitiveComponent Object Reference") (OtherBodyIndex :type Integer) (bFromSweep :type Boolean) (SweepResult :type "HitResult Structure (by ref)"))
  (cast `/Game/Blueprints/EnvironmentBlueprints/PenBlueprint` OtherActor)
  (set `self.InsidePen` true)
  (`self.Event RunAway`)
  (bind _asfirst_person_character (cast `/Game/FirstPersonBP/Blueprints/FirstPersonCharacter` (`GameplayStatics.GetPlayerCharacter` 0)))
  (bind _result (`/Engine/EditorBlueprintResources/StandardMacros.IncrementInt` (`/Game/FirstPersonBP/Blueprints/FirstPersonCharacter.PenPoints` _asfirst_person_character))
    (:`  `
      (if (== _result 15)
        (`KismetSystemLibrary.PrintString` "You Win")
        (else
          (`KismetSystemLibrary.PrintString` "Not YEt"))))))

(fn `UserConstructionScript`)