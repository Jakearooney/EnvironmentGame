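; Sheep AI Blueprint that flees from the first-person player character when it comes near.
; A Sphere component's overlap events track whether the player is inside the radius and start the flee on entry.
; RunAway uses AIMoveTo toward a point at a fixed distance directly away from the player, keeping the sheep's current height.
; The move re-triggers on success or failure for as long as the player stays inside.
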(event `self.ReceiveBeginPlay`
  (bind _asfirst_person_character (cast `/Game/FirstPersonBP/Blueprints/FirstPersonCharacter` (`GameplayStatics.GetPlayerCharacter` 0)))
  (set `self.CharacterRef` _asfirst_person_character))

(event `Event RunAway`
  (bind _returnvalue (`self.K2_GetActorLocation`))
  (bind _characterref (`self.CharacterRef`))
  (`/Engine/EditorBlueprintResources/StandardMacros.IsValid` _characterref
    (:`Is Valid`
      (`|AIMoveTo` self (`KismetMathLibrary.MakeVector` (.x (+ _returnvalue (* (`KismetMathLibrary.GetForwardVector` (`KismetMathLibrary.FindLookAtRotation` _returnvalue (`self.K2_GetActorLocation` _characterref))) -600.0))) (.y (+ _returnvalue (* (`KismetMathLibrary.GetForwardVector` (`KismetMathLibrary.FindLookAtRotation` _returnvalue (`self.K2_GetActorLocation` _characterref))) -600.0))) (.z _returnvalue)) null
        (:`OnSuccess`
          _)
        (:`OnFail`
          _))
      (if (`self.Inside Radius`)
        (`self.Event RunAway`)))))

(event `self.Sphere.OnComponentBeginOverlap`
  (params (OverlappedComponent :type "PrimitiveComponent Object Reference") (OtherActor :type "Actor Object Reference") (OtherComp :type "PrimitiveComponent Object Reference") (OtherBodyIndex :type Integer) (bFromSweep :type Boolean) (SweepResult :type "HitResult Structure (by ref)"))
  (cast `/Game/FirstPersonBP/Blueprints/FirstPersonCharacter` OtherActor)
  (set `self.Inside Radius` true)
  (`self.Event RunAway`))

(event `self.Sphere.OnComponentEndOverlap`
  (params (OverlappedComponent :type "PrimitiveComponent Object Reference") (OtherActor :type "Actor Object Reference") (OtherComp :type "PrimitiveComponent Object Reference") (OtherBodyIndex :type Integer))
  (cast `/Game/FirstPersonBP/Blueprints/FirstPersonCharacter` OtherActor)
  (set `self.Inside Radius` false))

(fn `UserConstructionScript`)